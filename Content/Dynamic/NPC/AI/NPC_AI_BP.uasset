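; AI controller for guard NPCs that runs the GuardBehaviour behavior tree on the PatrolData blackboard.
; AI Perception writes sensed actors not tagged "Enemy" to EnemyKey and clears the key when sensing is lost.
; Each tick, it sets the controlled ThirdPersonCharacter's AI aiming and shooting flags according to whether a focus actor exists.
; SetWaypointKey is an empty, unused leftover marked for removal.
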(event OnTargetPerceptionUpdated(AIPerception)
  (params (Actor :type Actor%20Object%20Reference) (Stimulus :type AI%20Stimulus%20Structure))
  (bind _enemykey (Variables|Default|GetEnemyKey))
  (bind _blackboardcompref (Variables|Default|GetBlackboardcompRef))
  ;[1 1 1] AI senses player and sets EnemyKey
  (if (not (Actor|ActorHasTag Actor "Enemy"))
    (if (.bSuccessfullySensed (Utilities|Struct|BreakAIStimulus Stimulus))
      (AI|Components|Blackboard|SetValueasObject _blackboardcompref _enemykey Actor)
      (else
        (AI|Components|Blackboard|ClearValue _blackboardcompref _enemykey)))))

(event EventBeginPlay
  (bind _blackboardcomponent (Class|AIController|UseBlackboard "/Game/Dynamic/NPC/AI/PatrolData.PatrolData"))
  (Variables|Default|SetBlackboardcompRef _blackboardcomponent)
  (AI|RunBehaviorTree "/Game/Dynamic/NPC/AI/GuardBehaviour.GuardBehaviour"))

(event EventTick
  (params (DeltaSeconds :type Float%20%28single-precision%29))
  (bind _returnvalue (Class|AIController|GetFocusActor))
  (bind _returnvalue_2 (Utilities|IsValid _returnvalue))
  ;[1 1 1] Set AI variables isShooting and AI isAiming if Focus Actor is Set
  (bind _asthird_person_character (Utilities|Casting|CastToThirdPersonCharacter (Pawn|GetControlledPawn)))
  (Variables|/Game/Dynamic/NPC/Behaviour/ThirdPersonCharacter.ThirdPersonCharacter_C|SetisAIAiming _asthird_person_character _returnvalue_2)
  (Variables|/Game/Dynamic/NPC/Behaviour/ThirdPersonCharacter.ThirdPersonCharacter_C|SetisAIShooting _asthird_person_character _returnvalue_2))

(fn ConstructionScript)

(fn SetWaypointKey
  (params (Blackboard%20Component :type Blackboard%20Component%20Object%20Reference)))