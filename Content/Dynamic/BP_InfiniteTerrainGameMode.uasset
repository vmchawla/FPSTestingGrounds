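; Game mode for an infinite terrain level that lays down the starting run of tiles and keeps the score.
; On BeginPlay it calls PopulateBoundsVolume, then repeatedly spawns BP_Tile actors, handing each the NavMeshActorPool.
; Each new tile's attach arrow location becomes the next spawn transform, chaining tiles end to end.
; AddToScore increments Score and prints it.
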(event EventBeginPlay
  (Class|InfiniteTerrainGameModeBase|PopulateBoundsVolume)
  (for _index (range 0 3)
    (CallFunction|SpawnTileandSetNextTileTransform)))

(fn ConstructionScript)

(fn SpawnTileandSetNextTileTransform
  (bind _returnvalue (Game|SpawnActorfromClass "/Game/Dynamic/Terrain/BP_Tile.BP_Tile_C" (Variables|Default|GetNextTileTransform) "Undefined" 0 0))
  (Class|Tile|SetPool _returnvalue (Variables|Default|GetNavMeshActorPool))
  (bind _arrow_transform (Default|GetAttachArrowLocation _returnvalue))
  (Variables|Default|SetNextTileTransform _arrow_transform))

(fn AddtoScore
  (bind _result (Math|Integer|IncrementInt (Variables|Default|GetScore))
    (:%20%20
      (Development|PrintString (Utilities|String|ToString(Integer) _result)))))